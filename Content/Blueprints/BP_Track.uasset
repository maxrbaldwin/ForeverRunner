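; BP_Track is an endless-runner floor tile with three lanes.
; On construction it adds an obstacle child actor at one of three spawn points and scatters coins inside a randomly chosen lane's box.
; Lane overlaps set BP_Runner's left/right movement flags, blocking moves past the outer lanes.
; The end trigger asks ThirdPersonGameMode to add a tile, then destroys this one after a short delay.
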(event OnComponentBeginOverlap(EndTrigger)
  (params (OtherActor :type Actor%20Object%20Reference) (OtherComp :type Primitive%20Component%20Object%20Reference) (OtherBodyIndex :type Integer) (bFromSweep :type Boolean) (SweepResult :type Hit%20Result%20Structure%20%28by%20ref%29))
  (Utilities|Casting|CastToBP_Runner OtherActor)
  (bind _asthird_person_game_mode (Utilities|Casting|CastToThirdPersonGameMode (Game|GetGameMode)))
  (Default|AddFloorTile _asthird_person_game_mode)
  (Utilities|FlowControl|Delay 2.0)
  (Actor|DestroyActor))

(event OnComponentBeginOverlap(TrackL)
  (params (OtherActor :type Actor%20Object%20Reference) (OtherComp :type Primitive%20Component%20Object%20Reference) (OtherBodyIndex :type Integer) (bFromSweep :type Boolean) (SweepResult :type Hit%20Result%20Structure%20%28by%20ref%29))
  (bind _asbp_runner (Utilities|Casting|CastToBP_Runner OtherActor))
  (Variables|/Game/ThirdPersonBP/Blueprints/BP_Runner.BP_Runner_C|SetcanMoveLeft _asbp_runner false))

(event OnComponentBeginOverlap(TrackR)
  (params (OtherActor :type Actor%20Object%20Reference) (OtherComp :type Primitive%20Component%20Object%20Reference) (OtherBodyIndex :type Integer) (bFromSweep :type Boolean) (SweepResult :type Hit%20Result%20Structure%20%28by%20ref%29))
  (bind _asbp_runner (Utilities|Casting|CastToBP_Runner OtherActor))
  (Variables|/Game/ThirdPersonBP/Blueprints/BP_Runner.BP_Runner_C|SetcanMoveRight _asbp_runner false))

(event OnComponentBeginOverlap(TrackM)
  (params (OtherActor :type Actor%20Object%20Reference) (OtherComp :type Primitive%20Component%20Object%20Reference) (OtherBodyIndex :type Integer) (bFromSweep :type Boolean) (SweepResult :type Hit%20Result%20Structure%20%28by%20ref%29))
  (bind _asbp_runner (Utilities|Casting|CastToBP_Runner OtherActor))
  (Variables|/Game/ThirdPersonBP/Blueprints/BP_Runner.BP_Runner_C|SetcanMoveLeft _asbp_runner true)
  (Variables|/Game/ThirdPersonBP/Blueprints/BP_Runner.BP_Runner_C|SetcanMoveRight _asbp_runner true))

(fn ConstructionScript
  (CallFunction|GetSpawnPoints)
  (CallFunction|SpawnRandomObstacle)
  (CallFunction|SpawnCoins))

(fn GetAttachTransform
  (return (Transformation|GetWorldTransform (Variables|Default|GetAttachPoint))))

(fn GetSpawnPoints
  (Variables|Default|SetOBSpawnPoints (Utilities|Array|MakeArray (Transformation|GetRelativeTransform (Variables|Default|GetSpawnPointR)) (Transformation|GetRelativeTransform (Variables|Default|GetSpawnPointL)) (Transformation|GetRelativeTransform (Variables|Default|GetSpawnPointM)))))

(fn SpawnRandomObstacle
  (AddComponent|AddChildActorComponent false (Utilities|Array|Get(acopy) (Variables|Default|GetOBSpawnPoints) (Math|Random|RandomInteger 3))))

(fn SpawnCoins
  (bind _randomtrack (Variables|Default|GetRandomTrack))
  (CallFunction|SetRandomTrack)
  (for _index (range 0 (Variables|Default|GettotalCoinsSpawned))
    (AddComponent|AddChildActorComponent false (Math|Conversions|ToTransform(Vector) (Math|Random|RandomPointinBoundingBox (Variables|/Script/Engine.SceneComponent|GetRelativeLocation _randomtrack) (Variables|/Script/Engine.BoxComponent|GetBoxExtent _randomtrack))))))

(fn SetRandomTrack
  (Variables|Default|SetRandomTrack (Utilities|Array|Get(acopy) (Utilities|Array|MakeArray (Variables|Default|GetTrackL) (Variables|Default|GetTrackR) (Variables|Default|GetTrackM)) (Math|Random|RandomIntegerinRange 0 2))))